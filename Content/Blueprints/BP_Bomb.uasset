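; BP_Bomb is a timed bomb tied to the player pawn that instigated it.
; BeginPlay starts a timer that destroys the actor after ExplosionDelay, and EndPlay then calls OnBombExploded on the instigating BP_PlayerPawn.
; Its sphere switches to blocking the Pawn channel once a player pawn stops overlapping it, so the bomb turns solid after the player steps off.
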(event `self.ReceiveBeginPlay`
  ;[1 1 1] Bomb lifecycle
  (`KismetSystemLibrary.K2_SetTimer` null "Destroy Bomb" (`self.ExplosionDelay`)))

(event `self.ReceiveEndPlay`
  (params (EndPlayReason :type "EEndPlayReason Enum" :default "Destroyed"))
  ;[1 1 1] Bomb lifecycle
  (bind _asbp_player_pawn (cast `/Game/Blueprints/BP_PlayerPawn` (`self.GetInstigator`)))
  (`/Game/Blueprints/BP_PlayerPawn.On Bomb Exploded` _asbp_player_pawn))

(event `Destroy Bomb`
  ;[1 1 1] Bomb lifecycle
  (`self.K2_DestroyActor`))

(event `self.Shape_Sphere.OnComponentEndOverlap`
  (params (OverlappedComponent :type "PrimitiveComponent Object Reference") (OtherActor :type "Actor Object Reference") (OtherComp :type "PrimitiveComponent Object Reference") (OtherBodyIndex :type Integer))
  ;[1 1 1] Physics enabling
  (cast `/Game/Blueprints/BP_PlayerPawn` OtherActor)
  (`PrimitiveComponent.SetCollisionResponseToChannel` (`self.Shape_Sphere`) "ECC_Pawn" "ECR_Block"))

(fn `UserConstructionScript`)