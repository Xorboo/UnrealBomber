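; BP_WallDestroyable is a wall Blueprint that can leave a random pickup behind when it leaves play.
; On EndPlay, a weighted roll against SpawnChance decides whether to spawn a class picked by RandomElement from PossiblePickups at the wall's transform.
; The EndPlay reason is not checked, so the roll is not limited to destruction.
; The construction script only calls its parent, and no destruction logic appears here.
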(event `self.ReceiveEndPlay`
  (params (EndPlayReason :type "EEndPlayReason Enum" :default "Destroyed"))
  ;[1 1 1] Spawn Random Pickup
  (if (`KismetMathLibrary.RandomBoolWithWeight` (`self.Spawn Chance`))
    (`|SpawnActorFromClass` (`self.Random Element` (`self.Possible Pickups`)) (`self.GetTransform`) "Undefined" "OverrideRootScale")))

(fn `UserConstructionScript`
  (`parent.UserConstructionScript`))