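; Player pawn for a Bomberman-style game that moves, plants bombs and handles death and respawn.
; Tick turns input into swept movement, rotating the capsule toward travel and sliding along blocking walls by projecting the remaining offset.
; Planting checks bomb stock and tile availability through UnrealBomberGameMode, spawns a grid-snapped bomb with extra range and registers it.
; Explosions refund bombs; death stops movement until a new match teleports the player back to start.
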(event `self.ReceiveBeginPlay`
  ;[1 1 1] Begin Play
  (`|ExecutionSequence`
    (:`then_0`
      (set `self.CurrentBombs` (`self.InitialBombs`)))
    (:`then_1`
      (set `self.CurrentSpeed` (`self.BaseSpeed`)))
    (:`then_2`
      (set `self.Initial Position` (`self.K2_GetActorLocation`)))))

(event `self.ReceiveTick`
  (params (DeltaSeconds :type "Float (single-precision)"))
  ;[1 1 1] Movement
  (bind _movement_vector (`self.Get Movement Vector` DeltaSeconds))
  (`self.Rotate Pawn` _movement_vector)
  (`self.Move Pawn` _movement_vector))

(event `InputAction|PlantBomb`
  (params (Key :type "Key Structure" :default "AnyKey"))
  ;[1 1 1] Bomb Spawning
  (:`Pressed`
    (bind _can_spawn (`self.CanSpawnBomb`))
    (if _can_spawn
      (`|ExecutionSequence`
        (:`then_0`
          (`/Engine/EditorBlueprintResources/StandardMacros.DecrementInt` (`self.CurrentBombs`)))
        (:`then_1`
          (bind _returnvalue (`self.Spawn Bomb`)))
        (:`then_2`
          (`self.Notify Game Mode` _returnvalue))))))

(event `On Bomb Exploded`
  ;[1 1 1] Bomb Destroyed
  (`/Engine/EditorBlueprintResources/StandardMacros.IncrementInt` (`self.CurrentBombs`)
    (:`  `
      (`AudioComponent.Play` (`self.Explosion_Cue`) 0.0))))

(event `OnPlayerDead`
  ;[1 1 1] Player Death
  (`AudioComponent.Play` (`self.Death_Sound`) 0.0)
  (set `self.IsPlayerDead` true))

(event `OnNeMatchStarted`
  ;[1 1 1] Player Respawn
  (if (`self.IsPlayerDead`)
    (set `self.IsPlayerDead` false)
    (`self.K2_SetActorLocation` (`self.Initial Position`) false true)))

(fn `CanSpawnBomb`
  (returns (`Can Spawn` :type Boolean))
  (bind _asunreal_bomber_game_mode (cast `/Game/Blueprints/UnrealBomberGameMode` (`GameplayStatics.GetGameMode`)))
  (bind _returnvalue (`UnrealBomberGameModeBase.IsFreeTile` _asunreal_bomber_game_mode (`self.K2_GetActorLocation`)))
  (return (and _returnvalue (`self.Has Bombs`))))

(fn `Get Movement Vector`
  (params (DeltaTime :type "Float (double-precision)"))
  (returns (`Movement Vector` :type "Vector Structure"))
  (return (* (* (`KismetMathLibrary.MakeVector` (`self.GetInputAxisValue`) (`self.GetInputAxisValue`)) (* (`KismetMathLibrary.Conv_BoolToInt` (not (`self.IsPlayerDead`))) (`self.CurrentSpeed`))) DeltaTime)))

(fn `Move Pawn`
  (params (DeltaLocation :type "Vector Structure"))
  (bind _sweephitresult (`self.K2_AddActorWorldOffset` DeltaLocation true))
  (bind (_bblockinghit _binitialoverlap _time _location _impactpoint _normal) (`GameplayStatics.BreakHitResult` _sweephitresult))
  (if _bblockinghit
    (`self.K2_AddActorWorldOffset` (* (`KismetMathLibrary.ProjectVectorOnToPlane` DeltaLocation (`KismetMathLibrary.Normal` (`KismetMathLibrary.MakeVector` (.x _normal) (.y _normal)))) (- 1.0 _time)) true)))

(fn `Notify Game Mode`
  (params (Bomb :type "BombBase Object Reference"))
  (bind _asunreal_bomber_game_mode (cast `/Game/Blueprints/UnrealBomberGameMode` (`GameplayStatics.GetGameMode`)))
  (`UnrealBomberGameModeBase.BombAdded` _asunreal_bomber_game_mode Bomb))

(fn `Rotate Pawn`
  (params (`Movement Vector` :type "Vector Structure"))
  (if (> (`KismetMathLibrary.VSizeSquared` `Movement Vector`) 0.0)
    (`SceneComponent.K2_SetWorldRotation` (`self.Shape_NarrowCapsule`) (`KismetMathLibrary.Conv_VectorToRotator` `Movement Vector`) false false)))

(fn `Spawn Bomb`
  (returns (ReturnValue :type "/Game/Blueprints/BP_Bomb Object Reference"))
  (bind _asunreal_bomber_game_mode (cast `/Game/Blueprints/UnrealBomberGameMode` (`GameplayStatics.GetGameMode`))
    (:`then`
      (bind _returnvalue (`UnrealBomberGameModeBase.RoundPositionToGrid` _asunreal_bomber_game_mode (`self.K2_GetActorLocation`)))
      (bind _returnvalue_2 (`|SpawnActorFromClass` (`self.Bomb`) (`KismetMathLibrary.Conv_VectorToTransform` _returnvalue) "Undefined" "OverrideRootScale"))
      (`BombBase.IncreaseBlastRadius` _returnvalue_2 (`self.BombExtraRange`)))
    (:`CastFailed`
      _))
  (return _returnvalue_2))

(fn `UserConstructionScript`)